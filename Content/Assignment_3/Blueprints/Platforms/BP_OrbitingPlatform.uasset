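; Platform Blueprint that moves its mesh along a circular path around its starting relative location.
; On BeginPlay it stores that origin, sets the timeline play rate from MoveSpeed and starts it.
; Each timeline update treats the track value as degrees, using cosine and sine scaled by Radius for the X and Y offsets.
; When the timeline finishes, it calls Play again rather than PlayFromStart.
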(event `self.ReceiveBeginPlay`
  (bind (_origin_x _origin_y) (`KismetMathLibrary.BreakVector` (`self.Origin`)))
  (set `self.Origin` (`SceneComponent.RelativeLocation` (`self.PlatformMesh`)))
  (`TimelineComponent.SetPlayRate` (`self.Moving Timeline`) (`self.MoveSpeed`))
  (bind (_direction _movetrack) (`Timeline|Moving Timeline`)
    (:`Update`
      (`SceneComponent.K2_SetRelativeLocation` (`self.PlatformMesh`) (`KismetMathLibrary.MakeVector` (+ (* (`KismetMathLibrary.DegCos` _movetrack) (`self.Radius`)) _origin_x) (+ _origin_y (* (`KismetMathLibrary.DegSin` _movetrack) (`self.Radius`)))) false false))
    (:`Finished`
      (`TimelineComponent.Play` (`self.Moving Timeline`)))))

(fn `UserConstructionScript`)