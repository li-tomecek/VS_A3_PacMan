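; BP_Ghost is a ghost enemy character that switches between patrol and chase movement speeds.
; The construction script creates a dynamic material for the ghost mesh, tinting its base color from a color map keyed by an enum.
; BeginPlay caches the player pawn for detection and compass use.
; PrepareToChase and PrepareToPatrol set the walk speed for each state, with no calls to them in this graph.
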(event `self.ReceiveBeginPlay`
  (set `self.PlayerRef` (`GameplayStatics.GetPlayerPawn` 0)) ; For detection and compass. Easier for each enemy to have a reference to the player rather than get it every frame
)

(fn `PrepareToChase`
  (set `CharacterMovementComponent.MaxWalkSpeed` (`self.MaxChaseSpeed`) (`self.CharacterMovement`)))

(fn `PrepareToPatrol`
  (set `CharacterMovementComponent.MaxWalkSpeed` (`self.MaxPatrolSpeed`) (`self.CharacterMovement`)))

(fn `UserConstructionScript`
  (bind _returnvalue (`KismetMaterialLibrary.CreateDynamicMaterialInstance` "/Game/Assignment_3/Blueprints/Enemies/Mesh/ghost_game_ready_texture_0_Mat.ghost_game_ready_texture_0_Mat"))
  (`MaterialInstanceDynamic.SetVectorParameterValue` _returnvalue "Base Color" (`BlueprintMapLibrary.Map_Find` (`self.ColorMap`) (`self.Color_Enum`)))
  (`PrimitiveComponent.SetMaterial` (`self.Ghost Mesh`) 0 _returnvalue))