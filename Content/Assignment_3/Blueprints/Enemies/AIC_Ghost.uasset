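; AI controller for the ghost enemy that runs the BT_Ghost behavior tree on BeginPlay.
; It contains sight logic chaining distance, view-cone and visibility-trace checks to set a player-tracking Blackboard key, with a timer delaying loss of tracking.
; That logic is disconnected: Tick is empty, and the view-cone angle calculation is unused, so the controller itself only starts the tree.
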(event `self.ReceiveBeginPlay`
  (`self.RunBehaviorTree` "/Game/Assignment_3/Blueprints/Enemies/BT_Ghost.BT_Ghost"))

(event `self.ReceiveTick`
  (params (DeltaSeconds :type "Float (single-precision)")))

(fn `Check For State Change`
  (params (Condition :type Boolean))
  (if Condition
    (if (not (`self.LastCheckedLOS`))
      (`BlackboardComponent.SetValueAsBool` (`self.Blackboard`) (`self.TrackingPlayerKey`) true) ; Then we just spotted the player.
      (set `self.LostVisionTimerActive` false))
    (elif (`self.LastCheckedLOS`)
      (set `self.LostVisionTimerActive` true) ; The we just lost the player. Start the timer
      (set `self.TimeRemaining` (`self.LostVisionDuration`)))))

(fn `Check LOS`
  (returns (`In LOS` :type Boolean))
  (locals (DistanceVector :type "Vector Structure"))
  (bind _output_get (set `local.DistanceVector` (- (`self.K2_GetActorLocation` (`GameplayStatics.GetPlayerPawn` 0)) (`self.K2_GetActorLocation` (`self.K2_GetPawn`)))))
  (if (<= (`KismetMathLibrary.VSize` _output_get) (`self.VisionDistance`))
    (if (<= (`KismetMathLibrary.DegAcos` (`KismetMathLibrary.Dot_VectorVector` (`KismetMathLibrary.Normal` (`local.DistanceVector`)) (`KismetMathLibrary.Normal` (`self.GetActorForwardVector` (`self.K2_GetPawn`))))) (`self.VisionHalfAngle`))
      (bind _outhit (`KismetSystemLibrary.LineTraceSingle` (`self.K2_GetActorLocation` (`self.K2_GetPawn`)) (`self.K2_GetActorLocation` (`GameplayStatics.GetPlayerPawn` 0)) "TraceTypeQuery1"))
      (cast `/Game/ThirdPerson/Blueprints/BP_ThirdPersonCharacter` (`.HitActor` (`GameplayStatics.BreakHitResult` _outhit)) ; 3. Check if first hit is to character and not wall
        (:`then`
          (return true))
        (:`CastFailed`
          (return false)))
      (else
        (return false)))
    (else
      (return false))))

(fn `UpdateTimer`
  (params (DetaTime :type "Float (double-precision)"))
  (set `self.TimeRemaining` (- (`self.TimeRemaining`) DetaTime)))

(fn `UserConstructionScript`
  (set `self.TimeRemaining` (`self.LostVisionDuration`)))