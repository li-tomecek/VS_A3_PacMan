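; BP_Collectible is a floating treasure pickup that awards score when the third-person character overlaps it.
; The construction script sets the mesh material from a map keyed by treasure type, and a self-restarting timeline bobs the mesh vertically.
; On overlap it spawns a collection effect, destroys itself, and passes the type's mapped value to BP_TreasureGameMode's CollectTreasure.
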(event `self.ReceiveBeginPlay`
  (bind (_direction _newtrack_0) (`Timeline|Height Timeline`)
    (:`Update`
      (`SceneComponent.K2_SetRelativeLocationAndRotation` :`self` (`self.CollectibleMesh`) :`NewLocation` (`KismetMathLibrary.MakeVector` 0.0 0.0 (* (`self.MaxHeightOffset`) _newtrack_0))))
    (:`Finished`
      (`TimelineComponent.Play` (`self.Height Timeline`)))))

(event `self.OverlapTrigger.OnComponentBeginOverlap`
  (params (OverlappedComponent :type "PrimitiveComponent Object Reference") (OtherActor :type "Actor Object Reference") (OtherComp :type "PrimitiveComponent Object Reference") (OtherBodyIndex :type Integer) (bFromSweep :type Boolean) (SweepResult :type "HitResult Structure (by ref)"))
  (cast `/Game/ThirdPerson/Blueprints/BP_ThirdPersonCharacter` OtherActor)
  (`self.StartFX`) ; Play Collection FX
  (bind _asbp_treasure_game_mode (cast `/Game/Assignment_1/Blueprints/BP_TreasureGameMode` (`GameplayStatics.GetGameMode`)))
  (`/Game/Assignment_1/Blueprints/BP_TreasureGameMode.CollectTreasure` _asbp_treasure_game_mode (`BlueprintMapLibrary.Map_Find` (`self.TreasureValues`) (`self.Treasure`))) ; Add treasure value to score baed on treasure type
)

(event `StartFX`
  (`NiagaraFunctionLibrary.SpawnSystemAtLocation` "/Game/Assignment_1/Blueprints/Collectibles/CollectibleEffect.CollectibleEffect" (`self.K2_GetActorLocation`) (struct) (0.6 0.6 0.6))
  (`self.K2_DestroyActor`))

(fn `UpdateTresureMaterial`
  (params (TreasureType :type Byte :default 0))
  (`PrimitiveComponent.SetMaterial` (`self.CollectibleMesh`) 0 (`BlueprintMapLibrary.Map_Find` (`self.TreasureMaterials`) (cast `/Game/Assignment_1/Blueprints/Collectibles/ETreasureType` TreasureType))))

(fn `UserConstructionScript`
  (`self.UpdateTresureMaterial` (`self.Treasure`)))