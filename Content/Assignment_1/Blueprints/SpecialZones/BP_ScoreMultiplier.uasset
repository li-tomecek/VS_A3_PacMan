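; BP_ScoreMultiplier is a powerup effect that changes the score multiplier in BP_TreasureGameMode.
; ApplyEffect runs the parent logic, then sets the game mode's multiplier to EffectMultiplier.
; It also registers itself in ActivePowerups and enables the matching overlay timer widget, using a hard-coded slot index for both.
; RemoveEffect restores the default multiplier before calling the parent, and leaves the slot and widget untouched.
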(fn `ApplyEffect`
  (`parent.ApplyEffect`)
  (bind _asbp_treasure_game_mode (cast `/Game/Assignment_1/Blueprints/BP_TreasureGameMode` (`GameplayStatics.GetGameMode`)))
  (`|ExecutionSequence`
    (:`then_0`
      (set `/Game/Assignment_1/Blueprints/BP_TreasureGameMode.ScoreMultiplier` (`self.EffectMultiplier`) _asbp_treasure_game_mode))
    (:`then_1`
      (`KismetArrayLibrary.Array_Set` (`/Game/Assignment_1/Blueprints/BP_TreasureGameMode.ActivePowerups` _asbp_treasure_game_mode) 1 self true) ; assign powerup to game mode
      (bind _gameoverlay (`/Game/Assignment_1/Blueprints/BP_TreasureGameMode.GameOverlay` _asbp_treasure_game_mode))
      (`/Game/Assignment_1/Blueprints/UI/WBP_GameOverlay.EnableWidget` _gameoverlay (`|GetArrayItem` (`/Game/Assignment_1/Blueprints/UI/WBP_GameOverlay.PowerupTimers` _gameoverlay) 1)) ; enable multiplier widget...ik hard coding array indices is bad
    )))

(fn `RemoveEffect`
  (bind _asbp_treasure_game_mode (cast `/Game/Assignment_1/Blueprints/BP_TreasureGameMode` (`GameplayStatics.GetGameMode`)))
  (set `/Game/Assignment_1/Blueprints/BP_TreasureGameMode.ScoreMultiplier` 1.0 _asbp_treasure_game_mode)
  (`parent.RemoveEffect`))

(fn `UserConstructionScript`
  (`parent.UserConstructionScript`))