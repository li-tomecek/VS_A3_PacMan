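; Speed boost powerup for the treasure game that temporarily raises the player character's max walk speed.
; ApplyEffect multiplies walk speed by EffectMultiplier only if no boost is active, so repeat pickups do not stack.
; It then registers itself in the game mode's ActivePowerups and enables the overlay timer widget, both through hardcoded slot indices.
; RemoveEffect divides the speed back before calling the parent.
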(fn `ApplyEffect`
  (`parent.ApplyEffect`)
  (bind _asbp_treasure_game_mode (cast `/Game/Assignment_1/Blueprints/BP_TreasureGameMode` (`GameplayStatics.GetGameMode`)))
  (`|ExecutionSequence`
    (:`then_0`
      (bind _activepowerups (`/Game/Assignment_1/Blueprints/BP_TreasureGameMode.ActivePowerups` _asbp_treasure_game_mode))
      (if (not (`KismetSystemLibrary.IsValid` (`|GetArrayItem` _activepowerups)))
        (bind _asbp_third_person_character (cast `/Game/ThirdPerson/Blueprints/BP_ThirdPersonCharacter` (`GameplayStatics.GetPlayerPawn` 0)))
        (bind _charactermovement (`Character.CharacterMovement` _asbp_third_person_character))
        (set `CharacterMovementComponent.MaxWalkSpeed` (* (`self.EffectMultiplier`) (`CharacterMovementComponent.MaxWalkSpeed` _charactermovement)) _charactermovement)))
    (:`then_1`
      (`KismetArrayLibrary.Array_Set` _activepowerups 0 self) ; assign powerup to Game Mode
      (bind _gameoverlay (`/Game/Assignment_1/Blueprints/BP_TreasureGameMode.GameOverlay` _asbp_treasure_game_mode))
      (`/Game/Assignment_1/Blueprints/UI/WBP_GameOverlay.EnableWidget` _gameoverlay (`|GetArrayItem` (`/Game/Assignment_1/Blueprints/UI/WBP_GameOverlay.PowerupTimers` _gameoverlay))) ; Enable speed boost widget....ik hardcoding array indices is bad
    )))

(fn `RemoveEffect`
  (bind _asbp_third_person_character (cast `/Game/ThirdPerson/Blueprints/BP_ThirdPersonCharacter` (`GameplayStatics.GetPlayerPawn` 0)))
  (bind _charactermovement (`Character.CharacterMovement` _asbp_third_person_character))
  (set `CharacterMovementComponent.MaxWalkSpeed` (/ (`CharacterMovementComponent.MaxWalkSpeed` _charactermovement) (`self.EffectMultiplier`)) _charactermovement)
  (`parent.RemoveEffect`))

(fn `UserConstructionScript`
  (`parent.UserConstructionScript`))